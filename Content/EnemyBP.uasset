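; Enemy character that wanders the navmesh, chases the player and can be grappled.
; Tick issues moves to random nearby reachable points, gated by a Moving flag, until PawnSensing sees a ThirdPersonCharacter.
; That sighting sets InRange, which is never cleared, and starts an AI move toward the player.
; BeginPlay enables grappling; LaunchSelf flings the enemy toward a location with a velocity-change impulse, while LaunchEndEvent adds only a zero impulse.
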(event OnSeePawn(PawnSensing)
  (params (Pawn :type Pawn%20Object%20Reference))
  (Variables|Default|SetInRange true)
  (bind _asthird_person_character (Utilities|Casting|CastToThirdPersonCharacter Pawn))
  (AI|AIMoveTo self "0, 0, 0" _asthird_person_character 5.0 false))

(event EventTick
  (params (DeltaSeconds :type Float%20%28single-precision%29))
  (if (not (Variables|Default|GetInRange))
    (if (not (Variables|Default|GetMoving))
      (AI|AIMoveTo self (.RandomLocation (Class|NavigationSystemV1|GetRandomPointinNavigableRadius (Transformation|GetActorLocation) 5e+02 0 0)) 0 5.0 false
        (:then
          (Variables|Default|SetMoving true))
        (:OnSuccess
          (Variables|Default|SetMoving false :!label _label))
        (:OnFail
          (goto _label))))))

(event Collision|EventActorBeginOverlap
  (params (OtherActor :type Actor%20Object%20Reference)))

(event EventBeginPlay
  (Variables|/Game/Grappling.Grappling_C|SetCanBeGrappled (Variables|Default|GetGrappling) true))

(fn ConstructionScript
  (|CallParentFunction))

(fn LaunchSelf
  (params (Location :type Vector) (GrappleSpeed :type Float%20%28single-precision%29))
  (Physics|AddImpulse (Variables|Character|GetCharacterMovement) (* (Math|Vector|Normalize (- Location (Transformation|GetActorLocation))) GrappleSpeed) true))

(fn LaunchEndEvent
  (Physics|AddImpulse (Variables|Character|GetCharacterMovement) "0, 0, 0" true))