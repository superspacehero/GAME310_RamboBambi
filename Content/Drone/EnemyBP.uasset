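; Enemy drone AI that roams the navmesh until the player is spotted, then chases and shoots.
; Pawn sensing feeds a shared EnemyManager, which holds the last known location and delayed alert all enemies follow.
; Tick drives movement, mesh aiming and extra downward force when falling, all paused while grappling.
; Grapple functions launch it toward a point, then stun it by zeroing walk speed; the sight reset is disconnected.
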(event OnSeePawn(PawnSensing)
  (params (Pawn :type Pawn%20Object%20Reference))
  (bind _enemymanager (Variables|Default|GetEnemyManager))
  ;[1 1 1] Seeing Player
  (bind _asthird_person_character (Utilities|Casting|CastToThirdPersonCharacter Pawn))
  (Variables|Default|SetCanSeePlayer true)
  (Variables|/Game/EnemyManger.EnemyManger_C|SetMostRecentLocation _enemymanager (Transformation|GetWorldLocation (Variables|/Game/ThirdPersonBP/Blueprints/ThirdPersonCharacter.ThirdPersonCharacter_C|GetTarget _asthird_person_character)))
  (Default|Seen _enemymanager)
  (if (not (Variables|/Game/EnemyManger.EnemyManger_C|GetPlayerSeen _enemymanager))
    (Class|PawnSensingComponent|SetPeripheralVisionAngle (Variables|Default|GetPawnSensing) 1.8e+02)
    (if (not (Variables|/Game/EnemyManger.EnemyManger_C|GetReporting _enemymanager))
      (CallFunction|SeenEvent)
      (Variables|/Game/EnemyManger.EnemyManger_C|SetReporting _enemymanager true))))

(event Custom|SeenEvent
  ;[1 1 1] Seen Event
  (Utilities|FlowControl|Delay 1.0)
  (Variables|/Game/EnemyManger.EnemyManger_C|SetPlayerSeen (Variables|Default|GetEnemyManager) true)
  (Class|PawnSensingComponent|SetPeripheralVisionAngle (Variables|Default|GetPawnSensing) (Variables|Default|GetOrigPeriph))
  (Audio|PlaySound2D "/Game/Audio/SFX/Files/Alert.Alert" 1.0 1.0 0.0 0 0))

(event Custom|Roam
  (AI|AIMoveTo 0 (.RandomLocation (Class|NavigationSystemV1|GetRandomPointinNavigableRadius (Transformation|GetActorLocation) 5e+02 0 0)) 0 5.0 false
    (:OnSuccess
      (Utilities|FlowControl|Delay 1.0)
      (Utilities|FlowControl|DoOnce false) ; enters at Reset
    )))

(event Custom|Stun
  (bind _charactermovement (Variables|Character|GetCharacterMovement))
  ;[1 1 1] Stun
  (Variables|Default|SetStunned true)
  (bind _output_get (Variables|/Script/Engine.CharacterMovementComponent|SetMaxWalkSpeed _charactermovement 0.0))
  (Development|PrintString (Utilities|String|ToString(Float) _output_get))
  (Utilities|FlowControl|Delay (Variables|Default|GetStunTime))
  (Variables|Default|SetStunned false)
  (Variables|/Script/Engine.CharacterMovementComponent|SetMaxWalkSpeed _charactermovement (Variables|Default|GetMoveSpeed)))

(event Custom|Shoot
  (bind _returnvalue (Transformation|GetActorLocation))
  (bind _capsulecomponent (Variables|Collision|GetCapsuleComponent))
  (bind _enemymanager (Variables|Default|GetEnemyManager))
  (bind _mostrecentlocation (Variables|/Game/EnemyManger.EnemyManger_C|GetMostRecentLocation _enemymanager))
  (bind (_x _y) (Math|Vector|BreakVector _mostrecentlocation))
  ;[1 1 1] Shoot
  (Transformation|SetWorldRotation _capsulecomponent (Math|Rotator|Lerp(Rotator) (Transformation|GetWorldRotation _capsulecomponent) (Math|Rotator|FindLookatRotation _returnvalue (Math|Vector|MakeVector _x _y (.Z (Math|Vector|BreakVector _returnvalue)))) (* (Utilities|Time|GetWorldDeltaSeconds) (Variables|Default|GetLookSpeed))) false false)
  (Utilities|FlowControl|DoOnce false :!label _label
    (:Completed
      (Game|SpawnActorfromClass "/Game/Bullet_Blueprint.Bullet_Blueprint_C" (Math|Transform|MakeTransform (Transformation|GetWorldLocation (Variables|Character|GetMesh)) (Transformation|GetActorRotation) "1.000000,0.100000,0.100000") "Undefined" 0 0)
      (Utilities|FlowControl|Delay (Variables|Default|GetShootCooldownTime))
      (goto _label Reset))))

(event Custom|SeePlayer
  (bind _returnvalue (Utilities|Time|GetWorldDeltaSeconds))
  (bind _lookspeed (Variables|Default|GetLookSpeed))
  (bind _mesh (Variables|Character|GetMesh))
  (bind _returnvalue_2 (* _returnvalue _lookspeed))
  (bind _relativerotation (Variables|/Script/Engine.SceneComponent|GetRelativeRotation _mesh))
  ;[1 1 1] See Player
  (if (Variables|Default|GetCanSeePlayer)
    (Transformation|SetRelativeRotation _mesh (Math|Rotator|MakeRotator (Math|Float|ClampAngle (.Roll (Math|Rotator|BreakRotator (Math|Rotator|Lerp(Rotator) _relativerotation (Math|Rotator|FindLookatRotation (Transformation|GetWorldLocation _mesh) (Variables|/Game/EnemyManger.EnemyManger_C|GetMostRecentLocation (Variables|Default|GetEnemyManager))) _returnvalue_2 true))) -6e+01 45.0) 0.0 2.7e+02) false false)
    (else
      (Transformation|SetRelativeRotation _mesh (Math|Rotator|Lerp(Rotator) _relativerotation "0,270.000000, 0" _returnvalue_2) false false))))

(event Custom|SeeReset
  (Utilities|FlowControl|DoOnce false :!label _label
    (:Completed
      (Variables|Default|SetCanSeePlayer false)
      (Utilities|FlowControl|Delay 1.0)
      (goto _label Reset))))

(event EventTick
  (params (DeltaSeconds :type Float%20%28single-precision%29))
  (bind _charactermovement (Variables|Character|GetCharacterMovement))
  (if (not (Variables|Default|GetIsGrappling))
    (CallFunction|SeePlayer)
    (if (AI|Components|NavMovement|IsFalling _charactermovement)
      (Physics|AddImpulse _charactermovement "0, 0,-5000.000000" false))
    (if (Variables|/Game/EnemyManger.EnemyManger_C|GetPlayerSeen (Variables|Default|GetEnemyManager))
      (AI|AIMoveTo self (Variables|/Game/EnemyManger.EnemyManger_C|GetMostRecentLocation (Variables|Default|GetEnemyManager)) 0 (Variables|Default|GetAttackRadius) false
        (:OnSuccess
          (CallFunction|Shoot)))
      (elif (not (Variables|Default|GetCanSeePlayer))
        (Utilities|FlowControl|DoOnce false
          (:Completed
            (CallFunction|Roam)))))))

(event EventBeginPlay
  ;[1 1 1] Begin
  (Variables|Default|SetPlayer (Game|GetPlayerController 0))
  (bind _outactors (Actor|GetAllActorsOfClass "/Game/EnemyManger.EnemyManger_C"))
  (Variables|Default|SetEnemyManager (Utilities|Array|Get(acopy) _outactors))
  (Variables|Default|SetOrigPeriph (Class|PawnSensingComponent|GetPeripheralVisionAngle (Variables|Default|GetPawnSensing)))
  (Variables|Default|SetMoveSpeed (Variables|/Script/Engine.CharacterMovementComponent|GetMaxWalkSpeed (Variables|Character|GetCharacterMovement))))

(fn ConstructionScript)

(fn LaunchSelf
  (params (Location :type Vector) (GrappleSpeed :type Float%20%28single-precision%29))
  (Physics|AddImpulse (Variables|Character|GetCharacterMovement) (* (Math|Vector|Normalize (- Location (+ (Transformation|GetActorLocation) "0, 0,200.000000"))) GrappleSpeed) true))

(fn LaunchEndEvent
  (Physics|AddImpulse (Variables|Character|GetCharacterMovement) "0, 0, 0" true)
  (CallFunction|Stun))